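; Base kickable cube that the player can kick around, destroyed with a death sound when it falls into a pit.
; An interface event passes the kick direction and airborne state to KickCube, which applies a velocity-change impulse to the cube.
; Ground kicks add strong lift and randomised spin, while jump kicks use a separate force with less relative lift and no added spin.
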(event `/Game/Jacks_BPs/MainGame/BPs/BPI_OnKicked.OnObjectKicked`
  (params (KickDirection :type "Vector Structure") (IsAirborne :type Boolean))
  ;[1 1 1] Interface picks up when cube has been kicked
  (`self.KickCube` KickDirection IsAirborne))

(event `/Game/Jacks_BPs/MainGame/BPs/BPI_OnDeathPitContact.FellIntoPit`
  ;[1 1 1] Play death noise and destroy cube when falling into pit
  (`GameplayStatics.PlaySoundAtLocation` "/Game/Jacks_BPs/Global/Audio/SFX/SFX_CubeDeath.SFX_CubeDeath" (`self.K2_GetActorLocation`) (struct) 0.2 1.0 0.0 "/Game/Jacks_BPs/Global/Audio/AttenuationSettings/CubeDeathAttenuation.CubeDeathAttenuation" null null null)
  (`self.K2_DestroyActor`))

(fn `KickCube`
  (params (KickDirection :type "Vector Structure") (PlayerAirborne :type Boolean))
  (locals (DirectionX :type "Float (double-precision)" :default 0.0) (DirectionY :type "Float (double-precision)" :default 0.0))
  (bind _kickforce (`self.KickForce`))
  (bind _jumpkickforce (`self.JumpKickForce`))
  (bind _returnvalue (* (`local.DirectionY`) _kickforce))
  (bind _returnvalue_2 (* 5.0 _kickforce))
  (bind _returnvalue_3 (* (`local.DirectionX`) _kickforce))
  (set `local.DirectionX` KickDirection_X)
  (set `local.DirectionY` KickDirection_Y)
  (if PlayerAirborne
    ;[1 1 1] On a jump kick, apply less lift and more power
    (`KismetSystemLibrary.PrintString` "WICKED JUMP KICK")
    (`PrimitiveComponent.AddImpulse` (`self.Cube`) (`KismetMathLibrary.MakeVector` (* (`local.DirectionX`) _jumpkickforce) (* (`local.DirectionY`) _jumpkickforce) (* 1.0 _jumpkickforce)) "None" true)
    (else
      ;[1 1 1] Apply force and rotation on kick
      (`PrimitiveComponent.AddImpulse` (`self.Cube`) (`KismetMathLibrary.MakeVector` _returnvalue_3 _returnvalue _returnvalue_2) "None" true)
      ;[1 1 1] Randomise the kick force for the rotation to give it some spice
      (bind _output_get (set `self.RandomRotationForce` (`KismetMathLibrary.MakeVector` (`KismetMathLibrary.RandomFloatInRange` (* _returnvalue_3 0.0) (* _returnvalue_3 1.0)) (`KismetMathLibrary.RandomFloatInRange` (* _returnvalue 0.0) (* _returnvalue 1.0)) (`KismetMathLibrary.RandomFloatInRange` (* _returnvalue_2 -0.25) (* _returnvalue_2 0.25)))))
      (`PrimitiveComponent.AddAngularImpulseInDegrees` (`self.Cube`) _output_get "None" true))))

(fn `UserConstructionScript`)