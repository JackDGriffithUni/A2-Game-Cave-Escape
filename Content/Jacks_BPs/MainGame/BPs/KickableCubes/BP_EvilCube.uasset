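; BP_EvilCube is a physics cube that hops along a navmesh path towards PathfindingTarget.
; On BeginPlay it builds the path once, randomising all but the last point for less optimal-looking movement, and draws debug spheres.
; A looping timer with a randomised start delay waits until the cube nearly stops, advances the node when close, then launches an upward impulse towards it, weaker at short range.
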(event `self.ReceiveBeginPlay`
  (`self.GeneratePath`)
  (for _array_element (`NavigationPath.PathPoints` (`self.PathData`))
    (`KismetSystemLibrary.DrawDebugSphere` _array_element 50.0 12 (struct :`R` 0.029236 :`G` 1.0 :`B` 0.080663 :`A` 1.0) 100.0 1.0))
  (`KismetSystemLibrary.K2_SetTimer` null "DirectionToNextNode" 1.0 true false 5.0 2.5))

(fn `DirectionToNextNode`
  (if (<= (`KismetMathLibrary.VSize` (`SceneComponent.GetComponentVelocity` (`self.Cube`))) 5.0)
    (set `self.IsHopping` false)
    (if (<= (`KismetMathLibrary.Vector_Distance` (`|GetArrayItem` (`NavigationPath.PathPoints` (`self.PathData`)) (`self.CurrentNode`)) (`self.K2_GetActorLocation`)) 100.0)
      (`/Engine/EditorBlueprintResources/StandardMacros.IncrementInt` (`self.CurrentNode`)
        (:`  `
          (set `self.CurrentHopsTowardsNode` 0))))
    (`self.HopTowardsPoint` (`|GetArrayItem` (`NavigationPath.PathPoints` (`self.PathData`)) (`self.CurrentNode`)))))

(fn `GeneratePath`
  (locals (RandomNodeVariance :type "Rotator Structure") (PathPoints :type "Array of Vector Structure"))
  (set `self.CurrentNode` 0)
  (bind _returnvalue (`NavigationSystemV1.FindPathToLocationSynchronously` (`self.K2_GetActorLocation`) (`self.PathfindingTarget`) (`self.GetOwner`) null))
  (bind _output_get (set `self.PathData` _returnvalue))
  (bind _pathpoints (`NavigationPath.PathPoints` _output_get))
  ;[1 1 1] Randomise each pathfinding node to make the cube's path feel less 'min-maxed'
  (for (_array_element _array_index) _pathpoints
    (if (!= _array_index (`KismetArrayLibrary.Array_LastIndex` _pathpoints))
      (bind (_randomlocation _returnvalue_2) (`NavigationSystemV1.K2_GetRandomReachablePointInRadius` _array_element 200.0 null null))
      (if _returnvalue_2
        (`KismetArrayLibrary.Array_Set` _pathpoints _array_index _randomlocation)
        (`KismetSystemLibrary.DrawDebugSphere` _randomlocation 100.0 12 (struct :`R` 0.026234 :`G` 1.0 :`A` 1.0) 200.0 3.0)))))

(fn `HopTowardsPoint`
  (params (Target :type "Vector Structure"))
  (locals (DirectionToHop :type "Rotator Structure"))
  (bind _returnvalue (`self.K2_GetActorLocation`))
  (if (not (`self.IsHopping`))
    (bind _output_get (set `local.DirectionToHop` (`KismetMathLibrary.FindLookAtRotation` _returnvalue Target)))
    (bind (_returnvalue_x _returnvalue_y) (`KismetMathLibrary.BreakVector` (`KismetMathLibrary.GetForwardVector` _output_get)))
    (`PrimitiveComponent.AddImpulse` (`self.Cube`) (* (`KismetMathLibrary.MakeVector` _returnvalue_x _returnvalue_y 1.0) (* (`self.JumpForce`) (`KismetMathLibrary.Lerp` 0.25 1.0 (`KismetMathLibrary.FClamp` (/ (`KismetMathLibrary.Vector_Distance` _returnvalue Target) 200.0))))) "None" true)
    (set `self.IsHopping` true)
    (`/Engine/EditorBlueprintResources/StandardMacros.IncrementInt` (`self.CurrentHopsTowardsNode`))))

(fn `UserConstructionScript`
  (`parent.UserConstructionScript`))