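; BP_PureCube is a kickable cube that expires after a randomised lifespan, set in OnCubeSpawn.
; A looping one-second timer counts down and recolours its dynamic material by remaining-life ratio, lerping from near black toward BaseButtonColour, opposite to the commented blue-to-black fade.
; On expiry it plays a death sound before destroying itself, or is destroyed instantly and silently on the MainMenu level.
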(event `OnCubeSpawn`
  (bind _maxcubelifespan (`self.MaxCubeLifespan`))
  ;[1 1 1] On spawn, set cube max lifetime, set up a dynamic material so the cube will fade to black, and run a timer that slowly depletes its lifetime
  ;;[1 1 1] Don't play cube death SFX while on the main menu
  (bind _returnvalue (`GameplayStatics.GetCurrentLevelName` true))
  (if (`KismetStringLibrary.EqualEqual_StrStr` _returnvalue "MainMenu")
    (set `self.IsMainGame` false))
  (set `self.TimeUntilDespawn` (`KismetMathLibrary.RandomFloatInRange` (* _maxcubelifespan 0.9) (* _maxcubelifespan 1.1)))
  (bind _returnvalue_2 (`PrimitiveComponent.CreateDynamicMaterialInstance` (`self.Cube`) 0 "/Game/Jacks_BPs/MainGame/Materials/M_KickableCubeMaterial.M_KickableCubeMaterial" "None"))
  (bind _returnvalue_3 (`KismetSystemLibrary.K2_SetTimerDelegate` (delegate `DeathClockTick`) 1.0 true)))

(event `DeathClockTick`
  (bind _timeuntildespawn (`self.TimeUntilDespawn`))
  (bind _cubedeathsfx (`self.CubeDeathSFX`))
  (bind (_returnvalue_r _returnvalue_g _returnvalue_b) (break `LinearColor` (`KismetMathLibrary.LinearColorLerp` (`self.BaseButtonColour`) (struct) (/ (`self.TimeUntilDespawn`) (`self.MaxCubeLifespan`)))))
  (`/Engine/EditorBlueprintResources/StandardMacros.DecrementFloat` _timeuntildespawn
    (:`  `
      (if (<= _timeuntildespawn 0.0)
        (if (`self.IsMainGame`)
          ;[1 1 1] Play cube death SFX and then destroy the cube once the SFX has finished playing
          (`KismetSystemLibrary.K2_PauseTimerHandle` (stale `OnCubeSpawn` _returnvalue_3))
          (if (not (`AudioComponent.IsPlaying` _cubedeathsfx))
            (`AudioComponent.Play` _cubedeathsfx 0.0)
            (`KismetSystemLibrary.Delay` (`SoundBase.Duration` (`AudioComponent.Sound` _cubedeathsfx)))
            (`self.K2_DestroyActor`) ; Destroy cube once lifetime expires and SFX finishes
          )
          (else
            (`self.K2_DestroyActor`) ; Destroy cube instantly when lifetime expires on the main menu
          ))
        (else
          ;[1 1 1] Slowly fade the cube from blue to black
          (`MaterialInstanceDynamic.SetVectorParameterValue` (stale `OnCubeSpawn` _returnvalue_2) "KickableCubeColour" (make `LinearColor` _returnvalue_r _returnvalue_g _returnvalue_b)))))))

(fn `UserConstructionScript`
  (`parent.UserConstructionScript`))