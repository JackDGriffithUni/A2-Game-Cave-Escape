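; BP_ExitDoor is the cave escape exit door that triggers the win when the player touches it while it is unlocked.
; On Hit, it checks that the other actor is player 0's pawn, then reads ExitUnlocked from GameState_CaveEscape.
; If unlocked, it calls WinStateReached on GM_CaveEscape and plays WinMusic.
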(event `self.ReceiveHit`
  (params (MyComp :type "PrimitiveComponent Object Reference") (Other :type "Actor Object Reference") (OtherComp :type "PrimitiveComponent Object Reference") (bSelfMoved :type Boolean) (HitLocation :type "Vector Structure") (HitNormal :type "Vector Structure") (NormalImpulse :type "Vector Structure") (Hit :type "HitResult Structure (by ref)"))
  ;[1 1 1] If exit is unlocked when touched, the player has won!
  (if (== Other (`GameplayStatics.GetPlayerPawn` 0))
    (bind _asgame_state_cave_escape (cast `/Game/Jacks_BPs/MainGame/BPs/GameState_CaveEscape` (`GameplayStatics.GetGameState`)))
    (if (`/Game/Jacks_BPs/MainGame/BPs/GameState_CaveEscape.ExitUnlocked` _asgame_state_cave_escape)
      (bind _asgm_cave_escape (cast `/Game/Jacks_BPs/MainGame/BPs/GM_CaveEscape` (`GameplayStatics.GetGameMode`)))
      (`/Game/Jacks_BPs/MainGame/BPs/GM_CaveEscape.WinStateReached` _asgm_cave_escape)
      (`AudioComponent.Play` (`self.WinMusic`) 0.0))))

(fn `UserConstructionScript`)