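; BP_CubeCollector is a goal zone in the Cave Escape game that destroys overlapping kickable cubes and shows how many are still needed.
; Until the quota is met, each cube plays a sound, decrements the counter and refreshes the text monitor.
; Meeting it unlocks code doors through the GameState and notifies the GameMode.
; UpdateCodeDisplay lets the same monitor show an indexed, coloured code entry.
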(event `self.ReceiveBeginPlay`
  ;[1 1 1] Update screen on game start
  (`TextRenderComponent.K2_SetText` (`self.TextRender`) (`KismetTextLibrary.Conv_StringToText` (`KismetStringLibrary.Concat_StrStr` "CUBES NEEDED: " (`KismetStringLibrary.Conv_IntToString` (`self.CubesNeeded`))))))

(event `self.ReceiveActorBeginOverlap`
  (params (OtherActor :type "Actor Object Reference"))
  (bind _textrender (`self.TextRender`))
  (bind _cubesneeded (`self.CubesNeeded`))
  ;[1 1 1] If cube enters zone, destroy it
  (if (== (`GameplayStatics.GetObjectClass` OtherActor) "/Game/Jacks_BPs/MainGame/BPs/KickableCubes/BP_KickableCubeBase.BP_KickableCubeBase_C")
    (`self.K2_DestroyActor` OtherActor)
    (if (not (`self.GoalReached`))
      (`AudioComponent.Play` (`self.ScoreSFX`) 0.0)
      ;[1 1 1] Update the monitor that says how many cubes are still needed
      (`/Engine/EditorBlueprintResources/StandardMacros.DecrementInt` (`self.CubesNeeded`)
        (:`  `
          (if (> _cubesneeded 0)
            (`TextRenderComponent.K2_SetText` _textrender (`KismetTextLibrary.Conv_StringToText` (`KismetStringLibrary.Concat_StrStr` "CUBES NEEDED: " (`KismetStringLibrary.Conv_IntToString` _cubesneeded))))
            (else
              (`TextRenderComponent.K2_SetText` _textrender (`self.AllCubesText`))
              ;[1 1 1] Unlock the button room proximity doors, and tell the game mode that the quota has been reached
              (set `self.GoalReached` true)
              (bind _asgame_state_cave_escape (cast `/Game/Jacks_BPs/MainGame/BPs/GameState_CaveEscape` (`GameplayStatics.GetGameState`)))
              (`/Game/Jacks_BPs/MainGame/BPs/GameState_CaveEscape.UnlockCodeDoors` _asgame_state_cave_escape)
              (bind _asgm_cave_escape (cast `/Game/Jacks_BPs/MainGame/BPs/GM_CaveEscape` (`GameplayStatics.GetGameMode`)))
              (`/Game/Jacks_BPs/MainGame/BPs/GM_CaveEscape.CubeQuotaReached` _asgm_cave_escape))))))))

(fn `UpdateCodeDisplay`
  (params (ColourName :type String) (Colour :type "LinearColor Structure") (CodeIndex :type Integer))
  (bind _textrender (`self.TextRender`))
  (`TextRenderComponent.SetTextRenderColor` _textrender (`KismetMathLibrary.Conv_LinearColorToColor` Colour))
  (`TextRenderComponent.K2_SetText` _textrender (`KismetTextLibrary.Conv_StringToText` (`KismetStringLibrary.Concat_StrStr` "#" (`KismetStringLibrary.Conv_IntToString` CodeIndex) ": " ColourName))))

(fn `UserConstructionScript`)