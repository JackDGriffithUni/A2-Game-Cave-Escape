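; BP_CodeButton is a step-on button with an assigned colour, reporting to the GM_CaveEscape game mode.
; When the player pawn overlaps its HitBox, it passes itself and its colour to the game mode's ButtonSteppedOn.
; A timed cooldown blocks repeat presses, as does an AlreadyActivated flag that the button reads but never sets itself.
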(event `self.HitBox.OnComponentBeginOverlap`
  (params (OverlappedComponent :type "PrimitiveComponent Object Reference") (OtherActor :type "Actor Object Reference") (OtherComp :type "PrimitiveComponent Object Reference") (OtherBodyIndex :type Integer) (bFromSweep :type Boolean) (SweepResult :type "HitResult Structure (by ref)"))
  (if (== OtherActor (`GameplayStatics.GetPlayerPawn` 0))
    (if (`self.OnCooldown`)
      _
      (elif (not (`self.AlreadyActivated`))
        (set `self.OnCooldown` true)
        (bind _asgm_cave_escape (cast `/Game/Jacks_BPs/MainGame/BPs/GM_CaveEscape` (`GameplayStatics.GetGameMode`)))
        (`/Game/Jacks_BPs/MainGame/BPs/GM_CaveEscape.ButtonSteppedOn` _asgm_cave_escape self (`self.AssignedColour`))
        (`KismetSystemLibrary.RetriggerableDelay` (`self.CooldownLength`))
        (set `self.OnCooldown` false)))))

(fn `UserConstructionScript`)