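; BP_EvilCubeSpawner is a spawner that places a BP_EvilCube in the game at a random entry from its SpawnPoints.
; It spawns a cube on BeginPlay, then another 30 to 60 seconds after each OnEvilCubeVictory event.
; Spawning adjusts the position to avoid collisions and skips the spawn if it still collides, with no retry.
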(event `self.ReceiveBeginPlay`
  (`self.SpawnEvilCube`))

(event `/Game/Jacks_BPs/MainGame/BPs/BPI_OnEvilCubeReachedGoal.OnEvilCubeVictory`
  (`KismetSystemLibrary.Delay` (`KismetMathLibrary.RandomFloatInRange` 30.0 60.0))
  (`self.SpawnEvilCube`))

(fn `SpawnEvilCube`
  (locals (SpawnPoint :type "Vector Structure"))
  (bind _output_get (set `local.SpawnPoint` (`KismetArrayLibrary.Array_Random` (`self.SpawnPoints`))))
  (`|SpawnActorFromClass` "/Game/Jacks_BPs/MainGame/BPs/KickableCubes/BP_EvilCube.BP_EvilCube_C" (`KismetMathLibrary.Conv_VectorToTransform` _output_get) "AdjustIfPossibleButDontSpawnIfColliding" "MultiplyWithRoot" null null))

(fn `UserConstructionScript`)