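; Game mode for a cave escape level, running its colour-code puzzle and the win and lose screens.
; BeginPlay builds a duplicate-free code by randomly trimming the available colour names, then deals those colours randomly to the code buttons.
; Reaching the cube quota starts a looping timer that cycles the code on the collector and lights proximity doors.
; Stepped-on buttons are checked in order: mistakes reset progress, and the full sequence unlocks the exit through the game state.
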(event `self.ReceiveBeginPlay`
  (bind _colourcode (`self.ColourCode`))
  ;[1 1 1] Generate a random 4-long colour combination from all AvailableColours. All AvailableColours keys (the colour names) are copied into ColourCode array, and then entries are randomly removed until the array's length is 4. This prevents duplicate colours in the code
  (bind _keys (`BlueprintMapLibrary.Map_Keys` (`self.AvailableColours`)))
  (bind _output_get (set `self.ColourCode` _keys))
  (while (> (`KismetArrayLibrary.Array_Length` _output_get) (`self.CodeLength`))
    (`KismetArrayLibrary.Array_Remove` (`self.ColourCode`) (`KismetMathLibrary.RandomIntegerInRange` 0 (`KismetArrayLibrary.Array_Length` _colourcode))))
  (for (_array_element _array_index) _colourcode
    (`KismetSystemLibrary.PrintString` (`KismetStringLibrary.Concat_StrStr` "Colour " (`KismetStringLibrary.Conv_IntToString` (+ _array_index 1)) " = " _array_element) true true (struct :`G` 0.66 :`B` 1.0 :`A` 1.0) 0.0))
  (bind _outactors (`GameplayStatics.GetAllActorsOfClass` "/Game/Jacks_BPs/MainGame/BPs/BP_CodeButton.BP_CodeButton_C"))
  (set `self.CodeButtons` _outactors)
  (`self.AssignColoursToButtons`))

(event `CubeQuotaReached`
  (bind _returnvalue (`GameplayStatics.GetActorOfClass` "/Game/Jacks_BPs/MainGame/BPs/BP_CubeCollector.BP_CubeCollector_C"))
  (set `self.CubeCollector` _returnvalue)
  (`KismetSystemLibrary.K2_SetTimer` null "DisplayColourCode" 2.5 true false 1.0 0.5)
  (bind _outactors (`GameplayStatics.GetAllActorsWithTag` "IsProxDoor"))
  (for _array_element _outactors
    (if (== (`GameplayStatics.GetObjectClass` _array_element) "/Game/Jacks_BPs/MainGame/BPs/BP_ProxDoors.BP_ProxDoors_C")
      (bind _asbp_prox_doors (cast `/Game/Jacks_BPs/MainGame/BPs/BP_ProxDoors` _array_element))
      (`/Game/Jacks_BPs/MainGame/BPs/BP_ProxDoors.TurnOnSpotlights` _asbp_prox_doors))))

(event `WinStateReached`
  (bind _returnvalue (`GameplayStatics.GetPlayerController` 0))
  ;[1 1 1] Display and handle both win and loss screens
  (bind _returnvalue_2 (`|CreateWidget` "/Game/Jacks_BPs/MainGame/UI/WinScreen.WinScreen_C" _returnvalue))
  (`UserWidget.AddToPlayerScreen` _returnvalue_2 0)
  (`GameplayStatics.SetGamePaused` true)
  (`WidgetBlueprintLibrary.SetInputMode_UIOnlyEx` _returnvalue _returnvalue_2 "DoNotLock" true)
  (set `PlayerController.bShowMouseCursor` true _returnvalue)
  (bind _foundwidgets (`WidgetBlueprintLibrary.GetAllWidgetsOfClass` "/Game/Jacks_BPs/MainGame/UI/OxygenBarUI.OxygenBarUI_C" :!label _label))
  (for _array_element _foundwidgets
    (`Widget.RemoveFromParent` _array_element)))

(event `LoseStateReached`
  (bind _returnvalue (`GameplayStatics.GetPlayerController` 0))
  ;[1 1 1] Display and handle both win and loss screens
  (bind _returnvalue_2 (`|CreateWidget` "/Game/Jacks_BPs/MainGame/UI/LoseScreen.LoseScreen_C" _returnvalue))
  (`UserWidget.AddToPlayerScreen` _returnvalue_2 0)
  (`GameplayStatics.SetGamePaused` true)
  (`WidgetBlueprintLibrary.SetInputMode_UIOnlyEx` _returnvalue _returnvalue_2 "DoNotLock" true)
  (set `PlayerController.bShowMouseCursor` true _returnvalue)
  (goto _label))

(fn `AssignColoursToButtons`
  (locals (ColoursRemaining :type "Array of String") (RandomColourIndex :type Integer) (RandomColourName :type String))
  (bind _coloursremaining (`local.ColoursRemaining`))
  (set `local.ColoursRemaining` (`self.ColourCode`))
  (for _array_element (`self.CodeButtons`)
    (bind _output_get (set `local.RandomColourIndex` (`.OutIndex` (`KismetArrayLibrary.Array_Random` _coloursremaining))))
    (bind _output_get_2 (set `local.RandomColourName` (`|GetArrayItem` _coloursremaining _output_get)))
    (bind _output_get_3 (set `/Game/Jacks_BPs/MainGame/BPs/BP_CodeButton.AssignedColour` _output_get_2 _array_element))
    (`LightComponent.SetLightColor` (`/Game/Jacks_BPs/MainGame/BPs/BP_CodeButton.CodeColourLight` _array_element) (`BlueprintMapLibrary.Map_Find` (`self.AvailableColours`) _output_get_3) true)
    (`KismetArrayLibrary.Array_Remove` (`local.ColoursRemaining`) (`local.RandomColourIndex`))))

(fn `ButtonSteppedOn`
  (params (Button :type "/Game/Jacks_BPs/MainGame/BPs/BP_CodeButton Object Reference") (ButtonColour :type String))
  (bind _returnvalue (`KismetArrayLibrary.Array_Length` (`self.CurrentlyInputCode`)))
  (bind _returnvalue_2 (`KismetArrayLibrary.Array_Length` (`self.ColourCode`)))
  (bind _returnvalue_3 (`KismetArrayLibrary.Array_Add` (`self.CurrentlyInputCode`) ButtonColour))
  (if (`KismetStringLibrary.EqualEqual_StrStr` (`|GetArrayItem` (`self.ColourCode`) _returnvalue_3) (`|GetArrayItem` (`self.CurrentlyInputCode`) _returnvalue_3))
    (`KismetSystemLibrary.PrintString` "Codes match!")
    (set `/Game/Jacks_BPs/MainGame/BPs/BP_CodeButton.AlreadyActivated` true Button)
    (if (== _returnvalue_2 _returnvalue)
      (`KismetSystemLibrary.PrintString` "YOU WIN")
      (bind _asgame_state_cave_escape (cast `/Game/Jacks_BPs/MainGame/BPs/GameState_CaveEscape` (`GameplayStatics.GetGameState`)))
      (`/Game/Jacks_BPs/MainGame/BPs/GameState_CaveEscape.UnlockExitDoor` _asgame_state_cave_escape)
      (else
        (`KismetSystemLibrary.PrintString` (`KismetStringLibrary.Concat_StrStr` "Keep going, " (`KismetStringLibrary.Conv_IntToString` _returnvalue) "/" (`KismetStringLibrary.Conv_IntToString` _returnvalue_2)))))
    (else
      (bind _outactors (`GameplayStatics.GetAllActorsOfClass` "/Game/Jacks_BPs/MainGame/BPs/BP_CodeButton.BP_CodeButton_C"))
      (for _array_element _outactors
        (set `/Game/Jacks_BPs/MainGame/BPs/BP_CodeButton.AlreadyActivated` false _array_element))
      (`KismetSystemLibrary.PrintString` "Codes don't match")
      (`KismetArrayLibrary.Array_Clear` (`self.CurrentlyInputCode`)))))

(fn `DisplayColourCode`
  (bind _codedisplayindex (`self.CodeDisplayIndex`))
  (bind _output (`|GetArrayItem` (`self.ColourCode`) _codedisplayindex))
  (if (> (`self.CodeDisplayIndex`) (- (`self.CodeLength`) 1))
    (set `self.CodeDisplayIndex` 0) ; Reset the index to 0 (first colour in code array)
  )
  (`/Game/Jacks_BPs/MainGame/BPs/BP_CubeCollector.UpdateCodeDisplay` (`self.CubeCollector`) _output (`BlueprintMapLibrary.Map_Find` (`self.AvailableColours`) _output) (+ _codedisplayindex 1))
  (`/Engine/EditorBlueprintResources/StandardMacros.IncrementInt` (`self.CodeDisplayIndex`)))

(fn `UserConstructionScript`)