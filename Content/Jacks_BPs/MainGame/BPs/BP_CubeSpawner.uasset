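; BP_CubeSpawner keeps the level stocked with BP_KickableCube actors, up to a MaxCubes limit.
; On BeginPlay a looping two-second timer calls SpawnNewCube, which counts every existing cube in the world via GetAllActorsOfClass.
; While below the cap, it spawns one cube at a random point inside the SpawnArea component's bounds, then gives it a random rotation and random angular impulse so it tumbles.
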(event `self.ReceiveBeginPlay`
  (`KismetSystemLibrary.K2_SetTimer` null "SpawnNewCube" 2.0 true))

(fn `SpawnNewCube`
  (bind _returnvalue (`KismetMathLibrary.RandomFloatInRange` -100.0 100.0))
  (bind (_origin _boxextent) (`KismetSystemLibrary.GetComponentBounds` (`self.SpawnArea`)))
  (bind _outactors (`GameplayStatics.GetAllActorsOfClass` "/Game/Jacks_BPs/MainGame/BPs/BP_KickableCube.BP_KickableCube_C"))
  (if (< (`KismetArrayLibrary.Array_Length` _outactors) (`self.MaxCubes`))
    (bind _returnvalue_2 (`|SpawnActorFromClass` "/Game/Jacks_BPs/MainGame/BPs/BP_KickableCube.BP_KickableCube_C" (`KismetMathLibrary.Conv_VectorToTransform` (`KismetMathLibrary.RandomPointInBoundingBox` _origin _boxextent)) "Undefined" "MultiplyWithRoot" null null))
    (`self.K2_SetActorRotation` _returnvalue_2 (`KismetMathLibrary.RandomRotator` true) true)
    (`PrimitiveComponent.AddAngularImpulseInDegrees` (`/Game/Jacks_BPs/MainGame/BPs/BP_KickableCube.Cube` _returnvalue_2) (`KismetMathLibrary.MakeVector` _returnvalue _returnvalue _returnvalue) "None" true)))

(fn `UserConstructionScript`)