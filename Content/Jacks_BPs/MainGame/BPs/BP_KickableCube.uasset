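; BP_KickableCube is a physics cube that can be kicked and destroys itself when its lifespan runs out.
; A looping one-second timer counts down the lifespan, darkening a dynamic material's colour from the base colour towards black before destroying the actor.
; KickCube applies a mass-independent impulse along the kick direction with added lift, plus a randomised angular impulse for spin.
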(event `self.ReceiveBeginPlay`
  (set `self.TimeUntilDespawn` (`self.CubeLifespan`))
  (bind _returnvalue (`PrimitiveComponent.CreateDynamicMaterialInstance` (`self.Cube`) 0 "/Game/Jacks_BPs/MainGame/Materials/M_KickableCubeMaterial.M_KickableCubeMaterial" "None"))
  (`KismetSystemLibrary.K2_SetTimerDelegate` (delegate `DeathClockTick`) 1.0 true))

(event `DeathClockTick`
  (bind _timeuntildespawn (`self.TimeUntilDespawn`))
  (bind (_returnvalue_r _returnvalue_g _returnvalue_b) (break `LinearColor` (`KismetMathLibrary.LinearColorLerp` (struct :`A` 0.996) (`self.BaseButtonColour`) (/ (`self.TimeUntilDespawn`) (`self.CubeLifespan`)))))
  (`/Engine/EditorBlueprintResources/StandardMacros.DecrementFloat` _timeuntildespawn
    (:`  `
      (if (<= _timeuntildespawn 0.0)
        (`self.K2_DestroyActor`)
        (else
          (`MaterialInstanceDynamic.SetVectorParameterValue` (stale `self.ReceiveBeginPlay` _returnvalue) "KickableCubeColour" (make `LinearColor` _returnvalue_r _returnvalue_g _returnvalue_b)))))))

(fn `KickCube`
  (params (KickDirection :type "Vector Structure"))
  (bind _kickforce (`self.KickForce`))
  (bind _returnvalue (* 2.5 _kickforce))
  (bind _returnvalue_2 (* KickDirection_X _kickforce))
  (bind _returnvalue_3 (* KickDirection_Y _kickforce))
  ;[1 1 1] Apply force and rotation on kick
  (`PrimitiveComponent.AddImpulse` (`self.Cube`) (`KismetMathLibrary.MakeVector` _returnvalue_2 _returnvalue_3 _returnvalue) "None" true)
  ;[1 1 1] Randomise the kick force for the rotation to give it some spice
  (bind _output_get (set `self.RandomRotationForce` (`KismetMathLibrary.MakeVector` (`KismetMathLibrary.RandomFloatInRange` (* _returnvalue_2 0.0) (* _returnvalue_2 1.0)) (`KismetMathLibrary.RandomFloatInRange` (* _returnvalue_3 0.0) (* _returnvalue_3 1.0)) (`KismetMathLibrary.RandomFloatInRange` (* _returnvalue -0.25) (* _returnvalue 0.25)))))
  (`PrimitiveComponent.AddAngularImpulseInDegrees` (`self.Cube`) _output_get "None" true))

(fn `UserConstructionScript`)