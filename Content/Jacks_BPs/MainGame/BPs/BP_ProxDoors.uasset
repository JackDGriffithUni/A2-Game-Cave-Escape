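; BP_ProxDoors is a proximity door that rises when the player pawn overlaps it, provided GameState_CaveEscape reports code doors unlocked.
; BeginPlay records the start position and a raised end position, which a Timeline lerps the Cube between using SetRelativeLocation, despite both being world-space values.
; A one-shot flag prevents retriggering, while dust particles run during the rise.
; TurnOnSpotlights reveals a spotlight, which hides when the door starts opening.
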(event `self.ReceiveBeginPlay`
  ;[1 1 1] Set start and end position for door lerp, based on where the door is at game start
  (bind _output_get (set `self.StartingPosition` (`self.K2_GetActorLocation`)))
  (set `self.EndPosition` (`KismetMathLibrary.MakeVector` (.x _output_get) (.y _output_get) (+ (.z _output_get) (`self.RaisedDoorHeight`)))))

(event `TurnOnSpotlights`
  ;[1 1 1] Enable the door spotlights
  (`SceneComponent.SetVisibility` (`self.SpotLight`) true false))

(event `self.ReceiveActorBeginOverlap`
  (params (OtherActor :type "Actor Object Reference"))
  ;[1 1 1] Check if conditions are met to open the door when the player enters its proximity
  (if (== OtherActor (`GameplayStatics.GetPlayerPawn` 0))
    (bind _asgame_state_cave_escape (cast `/Game/Jacks_BPs/MainGame/BPs/GameState_CaveEscape` (`GameplayStatics.GetGameState`)))
    (if (`/Game/Jacks_BPs/MainGame/BPs/GameState_CaveEscape.CodeDoorsUnlocked` _asgame_state_cave_escape)
      (if (not (`self.DoorRaising`))
        (`KismetSystemLibrary.PrintString` "Door raising")
        (set `self.DoorRaising` true)
        (`ActorComponent.Activate` (`self.DustParticles`) false)
        (`SceneComponent.SetVisibility` (`self.SpotLight`) false false)
        ;[1 1 1] Opens door based on lerp using a timeline
        (bind (_direction _door_raise) (`Timeline|Timeline`)
          (:`Update`
            (`SceneComponent.K2_SetRelativeLocation` (`self.Cube`) (`KismetMathLibrary.VLerp` (`self.StartingPosition`) (`self.EndPosition`) _door_raise) false true))
          (:`Finished`
            (`ActorComponent.Deactivate` (`self.DustParticles`))))))))

(fn `UserConstructionScript`)